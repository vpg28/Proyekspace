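; BP_Boss1 is a boss that marches sideways in fixed steps and can drop downward, in a Space Invaders-like pattern.
; BeginPlay runs an endless Delay-paced loop that steps left or right according to ChangeSide, and triggers a downward step when GoingDown is set.
; The three movement macros use MoveComponentTo to offset the root component.
; Neither flag is set within this Blueprint's graphs.
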(event Collision|EventActorBeginOverlap
  (params (OtherActor :type Actor%20Object%20Reference)))

(event EventTick
  (params (DeltaSeconds :type Float%20%28single-precision%29)))

(event EventBeginPlay
  (if (Variables|Default|GetGoingDown) :!label _label
    (Utilities|MovingDown
      (:Completed
        _)))
  (Utilities|MovingL)
  (Utilities|FlowControl|Delay 0.2)
  (if (Variables|Default|GetChangeSide) :!label _label_2
    (if (Variables|Default|GetGoingDown)
      (Utilities|MovingDown
        (:Completed
          _)))
    (Utilities|MovingR)
    (Utilities|FlowControl|Delay 0.2)
    (goto _label_2)
    (else
      (goto _label))))

(fn ConstructionScript)