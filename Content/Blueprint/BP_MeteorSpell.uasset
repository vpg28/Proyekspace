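; BP_MeteorSpell is a meteor spell actor that detects a surface below it and explodes on it.
; From BeginPlay, a Trace event casts a 300-unit Visibility line downward, re-calling itself after a short retriggerable delay instead of using Tick.
; On a blocking hit it spawns an emitter at the impact point, scaled by ExplosionSize, then destroys itself.
; The graph itself applies no movement or damage.
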(event Custom|Trace
  (bind _returnvalue (Transformation|GetActorLocation))
  (bind _outhit (Collision|LineTraceByChannel _returnvalue (- _returnvalue "0.000000,0.000000,300.000000") "TraceTypeQuery1" false 0 "None"))
  (if (.bBlockingHit (Collision|BreakHitResult _outhit))
    (Effects|SpawnEmitteratLocation 0 (.Location (Collision|BreakHitResult _outhit)) "0, 0, 0" (Variables|Default|GetExplosionSize))
    (Actor|DestroyActor)
    (else
      (Utilities|FlowControl|RetriggerableDelay 0.01)
      (CallFunction|Trace))))

(event EventBeginPlay
  (CallFunction|Trace))

(event Collision|EventActorBeginOverlap
  (params (OtherActor :type Actor%20Object%20Reference)))

(event EventTick
  (params (DeltaSeconds :type Float%20%28single-precision%29)))

(fn ConstructionScript)