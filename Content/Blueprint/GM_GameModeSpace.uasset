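; Game mode for the space game that manages menu widgets, weapon-piece placement and meteor strikes on the level 1 planet.
; BeginPlay creates the main menu, level and coming-soon widgets, exposed through display/remove events, and attaches three child actors to the planet at randomly picked weapon-piece locations.
; A looping timer, gated by MeteorOut, spawns meteor pawns high above the level's TargetPoints, cycling through them in turn.
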(event Custom|CastMeteor
  (bind _indexmeteor (Variables|Default|GetindexMeteor))
  (bind _targetpoints (Variables|Default|GetTargetPoints))
  (bind _returnvalue (Utilities|Array|Length _targetpoints))
  (bind _returnvalue_2 (Math|Integer|%(Integer) _indexmeteor _returnvalue))
  (bind _output (Utilities|Array|Get(acopy) _targetpoints _returnvalue_2))
  ;[1 1 1] Mengeluarkan Meteor sesuai dengan tempat target
  (if (Variables|Default|GetMeteorOut)
    (Utilities|IsValid _output
      (:Is%20Valid
        (bind _output_get (Variables|Default|SetMeteorLoc (Transformation|GetActorLocation _output)))
        (AI|SpawnAIFromClass "/Game/Blueprint/BP_MeteorSpell.BP_MeteorSpell_C" 0 (+ _output_get "0.000000,0.000000,2500.000000") "0, 0, 0" false 0)
        (Math|Integer|IncrementInt (Variables|Default|GetindexMeteor))))))

(event Custom|Display%20Coming%20Soon
  ;[1 1 1] Custom Event untuk menampilkan dan meremove User Interface
  (UserInterface|Viewport|AddtoViewport (Variables|Default|GetUI%20Coming%20Soon) 0))

(event Custom|Remove%20Main%20Menu
  ;[1 1 1] Custom Event untuk menampilkan dan meremove User Interface
  (Widget|RemovefromParent (Variables|Default|GetUI%20Main%20Menu)))

(event Custom|Display%20Level
  ;[1 1 1] Custom Event untuk menampilkan dan meremove User Interface
  (UserInterface|Viewport|AddtoViewport (Variables|Default|GetUI%20Level) 0))

(event Custom|Remove%20Coming%20Soon
  ;[1 1 1] Custom Event untuk menampilkan dan meremove User Interface
  (Widget|RemovefromParent (Variables|Default|GetUI%20Coming%20Soon)))

(event Custom|Remove%20Level
  ;[1 1 1] Custom Event untuk menampilkan dan meremove User Interface
  (Widget|RemovefromParent (Variables|Default|GetUI%20Level)))

(event Custom|Display%20Main%20Menu
  ;[1 1 1] Custom Event untuk menampilkan dan meremove User Interface
  (UserInterface|Viewport|AddtoViewport (Variables|Default|GetUI%20Main%20Menu) 0))

(event EventTick
  (params (DeltaSeconds :type Float%20%28single-precision%29)))

(event EventBeginPlay
  (Utilities|FlowControl|Sequence
    (:then_0
      ;[1 1 1] User interface
      (bind _returnvalue (UserInterface|CreateWidget "/Game/Asset_UI/UI_mainmenu/UI_Mainmenu.UI_Mainmenu_C"))
      (Variables|Default|SetUI%20Main%20Menu _returnvalue)
      (bind _returnvalue_2 (UserInterface|CreateWidget "/Game/Asset_UI/UI_level/UI_Level.UI_Level_C"))
      (Variables|Default|SetUI%20Level _returnvalue_2)
      (bind _returnvalue_3 (UserInterface|CreateWidget "/Game/Asset_UI/UI_ComingSoon/UI_ComingSoon.UI_ComingSoon_C"))
      (Variables|Default|SetUI%20Coming%20Soon _returnvalue_3))
    (:then_1
      ;[1 1 1] Merandom Location Kepingan Senjata
      (bind _outactors (Actor|GetAllActorsOfClass "/Game/Blueprint/PLANET_level1.PLANET_level1_C"))
      (Variables|Default|Setplanet (Utilities|Array|Get(acopy) _outactors))
      (for _index (range 0 2)
        (AddComponent|AddChildActorComponent (Variables|Default|Getplanet) false (Math|Transform|MakeTransform (Utilities|Array|Get(acopy) (Variables|Default|GetlocKeping) (Utilities|Array|Get(acopy) (Variables|Default|GetpilihanIndex) (Math|Random|RandomIntegerinRange 0 (Variables|Default|GetpilihanLength)))) "0, 0, 0" "1.000000,1.000000,1.000000"))))
    (:then_2
      ;[1 1 1] Mengambil Data Tempat Target Meteor jatuh
      (bind _outactors_2 (Actor|GetAllActorsOfClass "/Game/Blueprint/TargetPoint.TargetPoint_C"))
      (Variables|Default|SetTargetPoints _outactors_2))
    (:then_3
      ;[1 1 1] Mengeluarkan Meteor sesuai dengan tempat target
      (bind _asbp_astronaut (Utilities|Casting|CastToBP_Astronaut (Game|GetPlayerCharacter 0)))
      (Variables|Default|SetAstronaut _asbp_astronaut)
      (Utilities|Time|SetTimerbyEvent (delegate Custom|CastMeteor) 3.0 true))))

(fn ConstructionScript)