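; BP_GunPickup is a world pickup that lets the BP_Astronaut player collect a gun.
; Overlapping its collision box stores the astronaut, enables player input on the pickup and turns on custom depth rendering on the gun mesh.
; Leaving the box disables input and custom depth.
; While input is enabled, pressing E increments the astronaut's Gunn count and destroys the pickup.
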(event OnComponentBeginOverlap(BoxCollisionGun)
  (params (OverlappedComponent :type Primitive%20Component%20Object%20Reference) (OtherActor :type Actor%20Object%20Reference) (OtherComp :type Primitive%20Component%20Object%20Reference) (OtherBodyIndex :type Integer) (bFromSweep :type Boolean) (SweepResult :type Hit%20Result%20Structure%20%28by%20ref%29))
  (bind _asbp_astronaut (Utilities|Casting|CastToBP_Astronaut OtherActor))
  (Variables|Default|SetAstronaut _asbp_astronaut)
  (Input|EnableInput (Game|GetPlayerController 0))
  (Rendering|SetRenderCustomDepth (Variables|Default|GetGun) true))

(event OnComponentEndOverlap(BoxCollisionGun)
  (params (OverlappedComponent :type Primitive%20Component%20Object%20Reference) (OtherActor :type Actor%20Object%20Reference) (OtherComp :type Primitive%20Component%20Object%20Reference) (OtherBodyIndex :type Integer))
  (Utilities|Casting|CastToBP_Astronaut OtherActor)
  (Input|DisableInput (Game|GetPlayerController 0))
  (Rendering|SetRenderCustomDepth (Variables|Default|GetGun) false))

(event EventBeginPlay)

(event EventTick
  (params (DeltaSeconds :type Float%20%28single-precision%29)))

(event Input|KeyboardEvents|E
  (params (Key :type Key%20Structure :default "None"))
  (bind _astronaut (Variables|Default|GetAstronaut))
  (:Pressed
    (Variables|/Game/Blueprint/BP_Astronaut.BP_Astronaut_C|SetGunn _astronaut (+ (Variables|/Game/Blueprint/BP_Astronaut.BP_Astronaut_C|GetGunn _astronaut) 1))
    (Actor|DestroyActor)))

(fn ConstructionScript)